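; Airplane pawn that flies forward continuously while the player steers it with roll and pitch.
; Each tick spins the left and right propellers in opposite directions and feeds the actor's forward vector into movement input.
; Roll and Pitch axis events apply frame-time-scaled local rotation, so the flight direction follows the nose.
; Two earlier offset-based movement attempts remain unconnected.
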(event `self.ReceiveTick`
  (params (DeltaSeconds :type "Float (single-precision)"))
  (set `self.Delta Seconds` DeltaSeconds)
  (`|ExecutionSequence`
    (:`then_0`
      ;[1 1 1] 왼쪽 프로펠러 회전
      (`SceneComponent.K2_AddLocalRotation` (`self.Left`) (`KismetMathLibrary.MakeRotator` (* (`GameplayStatics.GetWorldDeltaSeconds`) (`self.PropellerRotateSpeed`))) false false))
    (:`then_1`
      ;[1 1 1] 오른쪽 프로펠러 회전
      (`SceneComponent.K2_AddLocalRotation` (`self.Right`) (`KismetMathLibrary.MakeRotator` (* (`GameplayStatics.GetWorldDeltaSeconds`) (`self.PropellerRotateSpeed`) -1.0)) false false))
    (:`then_2`
      ;[1 1 1] 비행기 이동3
      (`self.AddMovementInput` (`self.GetActorForwardVector`)))))

(event `InputAxis|Roll`
  (params (AxisValue :type "Float (single-precision)"))
  ;[1 1 1] 롤 회전
  (`self.K2_AddActorLocalRotation` (`KismetMathLibrary.MakeRotator` (* AxisValue 60.0 (`GameplayStatics.GetWorldDeltaSeconds`)))))

(event `InputAxis|Pitch`
  (params (AxisValue :type "Float (single-precision)"))
  ;[1 1 1] 피치 회전
  (`self.K2_AddActorLocalRotation` (`KismetMathLibrary.MakeRotator` 0.0 (* AxisValue 60.0 (`GameplayStatics.GetWorldDeltaSeconds`)))))

(fn `UserConstructionScript`)